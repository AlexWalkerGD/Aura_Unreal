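; BP_FadeActor is an actor whose mesh fades out and in through a material "Fade" parameter.
; The construction script caches the original materials and creates dynamic instances from the fade materials.
; FadeOut applies those instances and plays the Fade timeline, which FadeIn reverses.
; On finish, a value of one restores original materials and blocks the Visibility channel, while zero ignores it.
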(event Custom|FadeOut
  (CallFunction|SetMaterialInstance)
  (bind _fade (Timeline|Fade Play)
    (:Update
      (for _array_element (Variables|Default|GetDynamicMaterialsIntances)
        (Rendering|Material|SetScalarParameterValue _array_element "Fade" _fade :!class /Script/Engine.MaterialInstanceDynamic)))
    (:Finished
      (CallFunction|FadeFinished _fade))))

(event Custom|FadeIn
  (bind _fade (Timeline|Fade Reverse)
    (:Update
      (for _array_element (Variables|Default|GetDynamicMaterialsIntances)
        (Rendering|Material|SetScalarParameterValue _array_element "Fade" _fade :!class /Script/Engine.MaterialInstanceDynamic)))
    (:Finished
      (CallFunction|FadeFinished _fade))))

(event EventBeginPlay)

(fn ConstructionScript
  (Utilities|Array|Clear (Variables|Default|GetDynamicMaterialsIntances))
  (Variables|Default|SetOriginalMaterials (Rendering|Material|GetMaterials (Variables|Default|GetMesh)))
  (for _array_element (Variables|Default|GetFadeMaterialsInstances)
    (bind _returnvalue (Rendering|Material|CreateDynamicMaterialInstance _array_element "None" "None" :!class /Script/Engine.KismetMaterialLibrary))
    (Utilities|Array|AddUnique (Variables|Default|GetDynamicMaterialsIntances) _returnvalue)))

(fn SetMaterialInstance
  (for (_array_element _array_index) (Variables|Default|GetDynamicMaterialsIntances)
    (Rendering|Material|SetMaterial (Variables|Default|GetMesh) _array_index _array_element)))

(fn FadeFinished
  (params (Value :type Float%20%28double-precision%29))
  (if (>= Value 1.0)
    (CallFunction|ResetMaterials)
    (Collision|SetCollisionResponsetoChannel (Variables|Default|GetMesh) "ECC_Visibility" "ECR_Block")
    (elif (<= Value 0.0)
      (Collision|SetCollisionResponsetoChannel (Variables|Default|GetMesh) "ECC_Visibility" "ECR_Ignore"))))

(fn ResetMaterials
  (for (_array_element _array_index) (Variables|Default|GetOriginalMaterials)
    (Rendering|Material|SetMaterial (Variables|Default|GetMesh) _array_index _array_element)))